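; Base character Blueprint for the boxing game, driving combat actions through the Gameplay Ability System.
; Melee, jump, backward dodge and flying sword actions check busy flags, set a montage gameplay tag, then activate ability classes.
; The sword event spawns BP_FlySword facing its target and triggers its ability once.
; Damage plays a hurt montage while alive; HP widget and death logic are disconnected, leaving those events empty.
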(event Custom|MeleeAttack
  ;[1 1 1] MeleeAttack
  (if (not (Variables|Default|GetIsUsingMelee))
    (Variables|Default|SetCurrentGameplayTag "(TagName=\"Event.Montage.Shared.MeleeHit\")")
    (Abilities|TryActivateAbilitybyClass (Variables|Default|GetAbilitySystemComponent) (Variables|Default|GetMeleeAttack_GameplayAbilityClass) true)))

(event EventBeginPlay
  (Class|MyCharacterBase|InitBoxCollision)
  (Networking|SwitchHasAuthority
    (:Authority
      (Variables|Default|SetIsAuthority true))
    (:Remote
      (Variables|Default|SetIsAuthority false))))

(event Collision|EventActorBeginOverlap
  (params (OtherActor :type Actor%20Object%20Reference)))

(event Custom|OnDeathEvent)

(event Custom|DelayDeathEvent)

(event EventOnDamaged
  (params (DeltaValue :type Float%20%28single-precision%29))
  (Class|MyCharacterBase|OnHealthChanged 0.0)
  (bind _returnvalue (Class|MyCharacterBase|IsAlive))
  (if _returnvalue
    (Animation|Montage|PlayMontage (Variables|Character|GetMesh) "/Game/Boxing/Characters/Animations/Montage/Hurt.Hurt")))

(event EventOnHealthChanged
  (params (newHealth :type Float%20%28single-precision%29))
  (if (Variables|Default|GetIsAuthority)
    _))

(event Custom|CreateFlySwordEvent
  (params (location :type Vector) (TargetToFollow :type BP%20Character%20Base%20Object%20Reference))
  (Networking|SwitchHasAuthority
    (:Authority
      (Development|PrintString "Hello"))
    (:Remote
      (Development|PrintString "Hello")))
  (Game|SpawnActorfromClass "/Game/Boxing/Actors/Weapons/BP_FlySword.BP_FlySword_C" (Math|Transform|MakeTransform location (Math|Conversions|RotationFromXVector (- (Transformation|GetActorLocation TargetToFollow) location))) "AdjustIfPossibleButDontSpawnIfColliding" 0 self)
  (Utilities|FlowControl|DoOnce false
    (:Completed
      (CallFunction|ActivateFlySwordAbility))))

(fn ConstructionScript)

(fn ClearCollisionTargetArray
  (Utilities|Array|Clear (Variables|Default|GetCollisionTargetArray))
  (return))

(fn DoJump
  (bind _return (CallFunction|CanUseAbility))
  (if _return
    (Variables|Default|SetCurrentGameplayTag "(TagName=\"Event.Montage.Shared.Jump\")")
    (Variables|Default|SetIsJumping true)
    (Abilities|TryActivateAbilitybyClass (Variables|Default|GetAbilitySystemComponent) (Variables|Default|GetJump_GameplayAbilityClass) true)
    (return)))

(fn CanUseAbility
  (return (not (Variables|Default|GetIsUsingAbility))))

(fn StandingDodgeBackward
  (bind _return (CallFunction|CanUseAbility))
  (if _return
    (Variables|Default|SetCurrentGameplayTag "(TagName=\"Event.Montage.Shared.Dodge\")")
    (Variables|Default|SetIsDodging true)
    (bind _returnvalue (Abilities|TryActivateAbilitybyClass (Variables|Default|GetAbilitySystemComponent) "/Game/Boxing/Abilities/share/GA_StandingDodgeBackward.GA_StandingDodgeBackward_C" true))
    (return _returnvalue)
    (else
      (return false))))

(fn ActivateFlySwordAbility
  (Networking|SwitchHasAuthority
    (:Authority
      (Development|PrintString "Hello"))
    (:Remote
      (Development|PrintString "Hello")))
  (if (Variables|Default|GetIsusingMagic)
    (return false)
    (else
      (Variables|Default|SetCurrentGameplayTag "(TagName=\"Event.Montage.Shared.FlySword\")")
      (CallFunction|SetUsingMagic false)
      (if (not (Utilities|IsValid (Variables|Default|GetFlySwordAbility)))
        (Abilities|TryActivateAbilitybyClass (Variables|Default|GetAbilitySystemComponent) "/Game/Boxing/Abilities/share/GA_FlySword.GA_FlySword_C" true)
        (return true)))))

(fn SetUsingMelee
  (params (in :type Boolean))
  (Variables|Default|SetIsUsingMelee in))

(fn SetUsingMagic
  (params (in :type Boolean))
  (Variables|Default|SetIsusingMagic in))

(fn InsertAbilitytoArray
  (params (in :type GA%20Ability%20Base%20Object%20Reference))
  (bind _curabilityarray (Variables|Default|GetCurAbilityArray))
  (if (not (Utilities|Array|ContainsItem _curabilityarray in))
    (Utilities|Array|AddUnique _curabilityarray in)))

(fn DeleteAbilitytoArray
  (params (in :type GA%20Ability%20Base%20Object%20Reference))
  (bind _curabilityarray (Variables|Default|GetCurAbilityArray))
  (if (Utilities|Array|ContainsItem _curabilityarray in)
    (Utilities|Array|RemoveItem _curabilityarray in)))