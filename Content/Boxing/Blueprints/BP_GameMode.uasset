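; Boxing game mode that handles player spawning, death respawn and the game-over screen.
; PostLogin records controllers and uses a FlipFlop to alternate them between the first two PlayerStarts.
; On death it detaches the pawn, plays its death montage, then respawns the controller through 生成玩家, which has its own FlipFlop.
; Game over shows a result widget with UI-only input; spectator cleanup exists, but spectator spawning is unconnected.
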(event Custom|OnPlayerDeadEvent
  (params (transform :type Transform) (Chararcter :type BP%20Character%20Base%20Object%20Reference))
  (bind _playerctrls (Variables|Default|GetPlayerCtrls))
  (if (> (Utilities|Array|Length _playerctrls) 0)
    (for _array_element _playerctrls
      (if (== (Pawn|GetController Chararcter) _array_element)
        (Variables|Default|SetdiedPawn (Pawn|GetControlledPawn _array_element))
        (Class|Pawn|DetachfromControllerPendingDestroy (Pawn|GetControlledPawn _array_element))
        (bind _output_get (Variables|Default|SetdiedCtrl _array_element))))
    (bind _asbp_player_character (Utilities|Casting|CastToBP_PlayerCharacter (Variables|Default|GetdiedPawn)))
    (Animation|Montage|PlayMontage (Variables|/Script/Engine.Character|GetMesh _asbp_player_character) (Variables|/Script/Boxing.MyCharacterBase|GetDeathMontage _asbp_player_character)
      (:OnCompleted
        (CallFunction|生成玩家 _output_get)))))

(event EventBeginPlay
  (|CallParentFunction))

(event EventTick
  (params (DeltaSeconds :type Float%20%28single-precision%29))
  (|CallParentFunction DeltaSeconds))

(event EventPostLogin
  (params (NewPlayer :type Player%20Controller%20Object%20Reference))
  (Variables|Default|SetNew%20Player NewPlayer)
  (bind _outactors (Actor|GetAllActorsOfClass "/Script/Engine.PlayerStart"))
  (Variables|Default|SetStartSpotList _outactors)
  (if (> (Utilities|Array|Length (Variables|Default|GetStartSpotList)) 1)
    (Utilities|FlowControl|FlipFlop
      (:A
        (Class|GameModeBase|RestartPlayeratPlayerStart (Variables|Default|GetNew%20Player) (Utilities|Array|Get(acopy) (Variables|Default|GetStartSpotList))))
      (:B
        (Class|GameModeBase|RestartPlayeratPlayerStart (Variables|Default|GetNew%20Player) (Utilities|Array|Get(acopy) (Variables|Default|GetStartSpotList) 1))))
    (Utilities|Array|Add (Variables|Default|GetPlayerCtrls) (Variables|Default|GetNew%20Player))))

(event Custom|OnPlayerPossessed
  (bind _spectatorpawn (Variables|Default|GetSpectatorPawn))
  (Utilities|IsValid _spectatorpawn
    (:Is%20Valid
      (Actor|DestroyActor _spectatorpawn))))

(event Custom|OnGameOver
  (bind _returnvalue (UserInterface|CreateWidget "/Game/Boxing/UI/Menu/BP_WidgetGameOver.BP_WidgetGameOver_C"))
  (bind _output_get (Variables|Default|SetResultUI _returnvalue))
  (UserInterface|Viewport|AddtoViewport _output_get 0)
  (Variables|Default|SetIsGameoverShow true)
  (Input|SetInputModeUIOnly (Game|GetPlayerController 0) 0 "LockAlways"))

(fn ConstructionScript)

(fn 生成玩家
  (params (PlayerCtrl :type Player%20Controller%20Object%20Reference))
  (Utilities|FlowControl|FlipFlop
    (:A
      (Class|GameModeBase|RestartPlayeratPlayerStart PlayerCtrl (Utilities|Array|Get(acopy) (Variables|Default|GetStartSpotList))))
    (:B
      (Class|GameModeBase|RestartPlayeratPlayerStart PlayerCtrl (Utilities|Array|Get(acopy) (Variables|Default|GetStartSpotList) 1)))))