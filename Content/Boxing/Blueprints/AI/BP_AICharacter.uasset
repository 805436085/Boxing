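; BP_AICharacter is the AI boxer, tracking health and landing punches on player characters through the Gameplay Ability System.
; Health changes update the HP widget and, once at zero, hide it, detach the controller and change capsule collision.
; Melee notify events toggle per-hand hit boxes during attack windows.
; Overlaps send the current gameplay tag event to itself with the player as target, recording victims to prevent repeat hits per attack.
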(event EventBeginPlay
  (|CallParentFunction) ; 此节点被禁用，将不会被调用。\n从引脚连出引线来编译功能。
)

(event Collision|EventActorBeginOverlap
  (params (OtherActor :type Actor%20Object%20Reference))
  (|CallParentFunction OtherActor) ; 此节点被禁用，将不会被调用。\n从引脚连出引线来编译功能。
)

(event EventTick
  (params (DeltaSeconds :type Float%20%28single-precision%29))
  (|CallParentFunction DeltaSeconds) ; 此节点被禁用，将不会被调用。\n从引脚连出引线来编译功能。
)

(event EventOnHealthChanged
  (params (DeltaValue :type Float%20%28single-precision%29))
  (bind _attributeset (Variables|Default|GetAttributeSet))
  (bind _hp (Variables|Default|GetHP))
  (bind _returnvalue (UserInterface|GetUserWidgetObject _hp))
  (bind _health (Variables|/Script/Boxing.MyAttributeSet|GetHealth _attributeset))
  (bind _currentvalue (Utilities|Struct|BreakGameplayAttributeData _health))
  (bind _returnvalue_2 (+ DeltaValue _currentvalue))
  (if (> _returnvalue_2 0.0)
    (Variables|Default|SetTempHP _returnvalue_2)
    (Class|IHUD|SetHP(Message) _returnvalue (/ (Variables|Default|GetTempHP) (.CurrentValue (Utilities|Struct|BreakGameplayAttributeData (Variables|/Script/Boxing.MyAttributeSet|GetMaxHealth _attributeset)))))
    (else
      (Variables|Default|SetTempHP 0.0)
      (Class|IHUD|SetHP(Message) _returnvalue (/ (Variables|Default|GetTempHP) (.CurrentValue (Utilities|Struct|BreakGameplayAttributeData (Variables|/Script/Boxing.MyAttributeSet|GetMaxHealth _attributeset)))))))
  (Class|MyCharacterBase|UpdateHP (Variables|Default|GetTempHP))
  (bind _returnvalue_3 (CallFunction|IsAlive))
  (if (not _returnvalue_3)
    (Utilities|FlowControl|DoOnce false
      (:Completed
        (CallFunction|OnDeathEvent)))))

(event EventOnDeathEvent
  (Rendering|SetVisibility (Variables|Default|GetHP) false false)
  (Class|Pawn|DetachfromControllerPendingDestroy)
  (Collision|SetCollisionObjectType (Variables|Default|GetCapsuleComponent) "ECC_WorldDynamic"))

(event OnComponentBeginOverlap(HandBox_R)
  (params (OverlappedComponent :type Primitive%20Component%20Object%20Reference) (OtherActor :type Actor%20Object%20Reference) (OtherComp :type Primitive%20Component%20Object%20Reference) (OtherBodyIndex :type Integer) (bFromSweep :type Boolean) (SweepResult :type Hit%20Result%20Structure%20%28by%20ref%29))
  (bind _self self)
  (bind _currentgameplaytag (Variables|Default|GetCurrentGameplayTag))
  (bind _collisiontargetarray (Variables|Default|GetCollisionTargetArray))
  (if (and (!= OtherActor self) (Variables|Default|GetbIsAttacking))
    (bind _asbp_player_character_base (Utilities|Casting|CastToBP_PlayerCharacterBase OtherActor))
    (Variables|Default|SetTargetActor _asbp_player_character_base)
    ;[1 1 1] 防穿模重入同一对象，本次攻击结束后清除
    (if (not (Utilities|Array|ContainsItem _collisiontargetarray (Variables|Default|GetTargetActor)))
      (Utilities|Array|Add _collisiontargetarray (Variables|Default|GetTargetActor))
      (Utilities|FlowControl|DoOnce false
        (:Completed
          (Ability|SendGameplayEventtoActor _self _currentgameplaytag (Utilities|Struct|MakeGameplayEventData _currentgameplaytag _self (Variables|Default|GetTargetActor)))
          (Development|PrintString "R"))))))

(event OnComponentBeginOverlap(HandBox_L)
  (params (OverlappedComponent :type Primitive%20Component%20Object%20Reference) (OtherActor :type Actor%20Object%20Reference) (OtherComp :type Primitive%20Component%20Object%20Reference) (OtherBodyIndex :type Integer) (bFromSweep :type Boolean) (SweepResult :type Hit%20Result%20Structure%20%28by%20ref%29))
  (bind _self self)
  (bind _collisiontargetarray (Variables|Default|GetCollisionTargetArray))
  (bind _currentgameplaytag (Variables|Default|GetCurrentGameplayTag))
  (if (and (!= OtherActor self) (Variables|Default|GetbIsAttacking))
    (bind _asbp_player_character_base (Utilities|Casting|CastToBP_PlayerCharacterBase OtherActor))
    (Variables|Default|SetTargetActor _asbp_player_character_base)
    ;[1 1 1] 防穿模重入同一对象，本次攻击结束后清除
    (if (not (Utilities|Array|ContainsItem _collisiontargetarray (Variables|Default|GetTargetActor)))
      (Utilities|Array|Add _collisiontargetarray (Variables|Default|GetTargetActor))
      (Utilities|FlowControl|DoOnce false
        (:Completed
          (Ability|SendGameplayEventtoActor _self _currentgameplaytag (Utilities|Struct|MakeGameplayEventData _currentgameplaytag _self (Variables|Default|GetTargetActor)))
          (Development|PrintString "L"))))))

(event OnComponentEndOverlap(HandBox_R)
  (params (OverlappedComponent :type Primitive%20Component%20Object%20Reference) (OtherActor :type Actor%20Object%20Reference) (OtherComp :type Primitive%20Component%20Object%20Reference) (OtherBodyIndex :type Integer))
  (bind _self self)
  (bind _currentgameplaytag (Variables|Default|GetCurrentGameplayTag))
  (Utilities|Casting|CastToBP_PlayerCharacterBase OtherActor)
  (Utilities|FlowControl|DoOnce false) ; enters at Reset
)

(event OnComponentEndOverlap(HandBox_L)
  (params (OverlappedComponent :type Primitive%20Component%20Object%20Reference) (OtherActor :type Actor%20Object%20Reference) (OtherComp :type Primitive%20Component%20Object%20Reference) (OtherBodyIndex :type Integer))
  (bind _self self)
  (bind _currentgameplaytag (Variables|Default|GetCurrentGameplayTag))
  (Utilities|Casting|CastToBP_PlayerCharacterBase OtherActor)
  (Utilities|FlowControl|DoOnce false) ; enters at Reset
)

(event EventInitBoxCollision
  (bind _boxarray (Variables|Default|GetBoxArray))
  (Utilities|Array|Add _boxarray (Variables|Default|GetHandBox_L))
  (Utilities|Array|Add _boxarray (Variables|Default|GetHandBox_R))
  (for _array_element _boxarray
    (Collision|SetCollisionEnabled _array_element "NoCollision")))

(event EventNotifyBeginonMeleeAttack
  (Variables|Default|SetbIsAttacking true)
  (for _array_element (Variables|Default|GetBoxArray)
    (Collision|SetCollisionEnabled _array_element "QueryOnly")))

(event EventNotifyEndonMeleeAttack
  (Variables|Default|SetbIsAttacking false)
  (for _array_element (Variables|Default|GetBoxArray)
    (Collision|SetCollisionEnabled _array_element "NoCollision")
    (CallFunction|ClearCollisionTargetArray)))

(event EventNotifyBeginonMeleeAttackLeftHand
  (Variables|Default|SetbIsAttacking true)
  (Collision|SetCollisionEnabled (Variables|Default|GetHandBox_L) "QueryOnly"))

(event EventNotifyEndonMeleeAttackLeftHand
  (Variables|Default|SetbIsAttacking false)
  (Collision|SetCollisionEnabled (Variables|Default|GetHandBox_L) "NoCollision")
  (CallFunction|ClearCollisionTargetArray))

(event EventNotifyBeginonMeleeAttackRightHand
  (Variables|Default|SetbIsAttacking true)
  (Collision|SetCollisionEnabled (Variables|Default|GetHandBox_R) "QueryOnly"))

(event EventNotifyEndonMeleeAttackRightHand
  (Variables|Default|SetbIsAttacking false)
  (Collision|SetCollisionEnabled (Variables|Default|GetHandBox_R) "NoCollision")
  (CallFunction|ClearCollisionTargetArray))

(fn ConstructionScript
  (|CallParentFunction))