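; Player boxer character that performs GAS-driven melee combos and reports health and SP to the player HUD.
; MeleeAttack activates GA_PlayerMelee, or jumps to a random next montage section while the combo window is open.
; Attack notify events toggle hand collision boxes, whose overlaps with AI characters send a gameplay event to itself, de-duplicated per swing.
; SP refreshes on the widget every Tick, while health updates through OnHealthChanged.
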(event EventBeginPlay
  (|CallParentFunction))

(event Collision|EventActorBeginOverlap
  (params (OtherActor :type Actor%20Object%20Reference))
  (|CallParentFunction OtherActor) ; 此节点被禁用，将不会被调用。\n从引脚连出引线来编译功能。
)

(event EventTick
  (params (DeltaSeconds :type Float%20%28single-precision%29))
  (|CallParentFunction DeltaSeconds)
  (Class|MyCharacterBase|UpdateStatus))

(event EventNotifyBeginonMeleeAttack
  (Variables|Default|SetbIsAttacking true)
  (for _array_element (Variables|Default|GetBoxArray)
    (Collision|SetCollisionEnabled _array_element "QueryOnly")))

(event EventNotifyEndonMeleeAttack
  (Variables|Default|SetbIsAttacking false)
  (for _array_element (Variables|Default|GetBoxArray)
    (Collision|SetCollisionEnabled _array_element "NoCollision")
    (CallFunction|ClearCollisionTargetArray)))

(event EventNotifyBeginonMeleeAttackLeftHand
  (Variables|Default|SetbIsAttacking true)
  (Collision|SetCollisionEnabled (Variables|Default|GetHandBox_L) "QueryOnly"))

(event EventNotifyEndonMeleeAttackLeftHand
  (Variables|Default|SetbIsAttacking false)
  (Collision|SetCollisionEnabled (Variables|Default|GetHandBox_L) "NoCollision")
  (CallFunction|ClearCollisionTargetArray))

(event EventNotifyBeginonMeleeAttackRightHand
  (Variables|Default|SetbIsAttacking true)
  (Collision|SetCollisionEnabled (Variables|Default|GetHandBox_R) "QueryOnly"))

(event EventNotifyEndonMeleeAttackRightHand
  (Variables|Default|SetbIsAttacking false)
  (Collision|SetCollisionEnabled (Variables|Default|GetHandBox_R) "NoCollision")
  (CallFunction|ClearCollisionTargetArray))

(event OnComponentBeginOverlap(HandBox_R)
  (params (OverlappedComponent :type Primitive%20Component%20Object%20Reference) (OtherActor :type Actor%20Object%20Reference) (OtherComp :type Primitive%20Component%20Object%20Reference) (OtherBodyIndex :type Integer) (bFromSweep :type Boolean) (SweepResult :type Hit%20Result%20Structure%20%28by%20ref%29))
  (bind _self self)
  (bind _currentgameplaytag (Variables|Default|GetCurrentGameplayTag))
  (bind _collisiontargetarray (Variables|Default|GetCollisionTargetArray))
  (if (and (!= OtherActor self) (Variables|Default|GetbIsAttacking))
    (bind _asbp_aicharacter_base (Utilities|Casting|CastToBP_AICharacterBase OtherActor))
    (Variables|Default|SetTargetActor _asbp_aicharacter_base)
    ;[1 1 1] 防穿模重入同一对象，本次攻击结束后清除
    (if (not (Utilities|Array|ContainsItem _collisiontargetarray (Variables|Default|GetTargetActor)))
      (Utilities|Array|Add _collisiontargetarray (Variables|Default|GetTargetActor))
      (Utilities|FlowControl|DoOnce false
        (:Completed
          (Ability|SendGameplayEventtoActor _self _currentgameplaytag (Utilities|Struct|MakeGameplayEventData _currentgameplaytag _self (Variables|Default|GetTargetActor)))
          (Development|PrintString "R"))))))

(event OnComponentBeginOverlap(HandBox_L)
  (params (OverlappedComponent :type Primitive%20Component%20Object%20Reference) (OtherActor :type Actor%20Object%20Reference) (OtherComp :type Primitive%20Component%20Object%20Reference) (OtherBodyIndex :type Integer) (bFromSweep :type Boolean) (SweepResult :type Hit%20Result%20Structure%20%28by%20ref%29))
  (bind _self self)
  (bind _collisiontargetarray (Variables|Default|GetCollisionTargetArray))
  (bind _currentgameplaytag (Variables|Default|GetCurrentGameplayTag))
  (if (and (!= OtherActor self) (Variables|Default|GetbIsAttacking))
    (bind _asbp_aicharacter_base (Utilities|Casting|CastToBP_AICharacterBase OtherActor))
    (Variables|Default|SetTargetActor _asbp_aicharacter_base)
    ;[1 1 1] 防穿模重入同一对象，本次攻击结束后清除
    (if (not (Utilities|Array|ContainsItem _collisiontargetarray (Variables|Default|GetTargetActor)))
      (Utilities|Array|Add _collisiontargetarray (Variables|Default|GetTargetActor))
      (Utilities|FlowControl|DoOnce false
        (:Completed
          (Ability|SendGameplayEventtoActor _self _currentgameplaytag (Utilities|Struct|MakeGameplayEventData _currentgameplaytag _self (Variables|Default|GetTargetActor)))
          (Development|PrintString "L"))))))

(event OnComponentEndOverlap(HandBox_R)
  (params (OverlappedComponent :type Primitive%20Component%20Object%20Reference) (OtherActor :type Actor%20Object%20Reference) (OtherComp :type Primitive%20Component%20Object%20Reference) (OtherBodyIndex :type Integer))
  (bind _self self)
  (bind _currentgameplaytag (Variables|Default|GetCurrentGameplayTag))
  (Utilities|Casting|CastToBP_AICharacterBase OtherActor)
  (Utilities|FlowControl|DoOnce false) ; enters at Reset
)

(event OnComponentEndOverlap(HandBox_L)
  (params (OverlappedComponent :type Primitive%20Component%20Object%20Reference) (OtherActor :type Actor%20Object%20Reference) (OtherComp :type Primitive%20Component%20Object%20Reference) (OtherBodyIndex :type Integer))
  (bind _self self)
  (bind _currentgameplaytag (Variables|Default|GetCurrentGameplayTag))
  (Utilities|Casting|CastToBP_AICharacterBase OtherActor)
  (Utilities|FlowControl|DoOnce false) ; enters at Reset
)

(event EventInitBoxCollision
  (bind _boxarray (Variables|Default|GetBoxArray))
  (Utilities|Array|Add _boxarray (Variables|Default|GetHandBox_L))
  (Utilities|Array|Add _boxarray (Variables|Default|GetHandBox_R))
  (for _array_element _boxarray
    (Collision|SetCollisionEnabled _array_element "NoCollision")))

(event EventUpdateStatus
  (bind _attributeset (Variables|Default|GetAttributeSet))
  (bind _asbp_player_controller (Utilities|Casting|CastToBP_PlayerController (Pawn|GetController)))
  (Default|SetSP (Variables|/Game/Boxing/Blueprints/Player/BP_PlayerController.BP_PlayerController_C|GetWidget_Player_PC _asbp_player_controller) (/ (.CurrentValue (Utilities|Struct|BreakGameplayAttributeData (Variables|/Script/Boxing.MyAttributeSet|GetSP _attributeset))) (.CurrentValue (Utilities|Struct|BreakGameplayAttributeData (Variables|/Script/Boxing.MyAttributeSet|GetMaxSP _attributeset))))))

(event EventOnHealthChanged
  (params (DeltaValue :type Float%20%28single-precision%29))
  (bind _attributeset (Variables|Default|GetAttributeSet))
  (bind _widgetplayerpc (Variables|Default|GetWidgetPlayerPC))
  (bind _health (Variables|/Script/Boxing.MyAttributeSet|GetHealth _attributeset))
  (bind _currentvalue (Utilities|Struct|BreakGameplayAttributeData _health))
  (bind _returnvalue (+ DeltaValue _currentvalue))
  (if (> _returnvalue 0.0)
    (Variables|Default|SetTempHP _returnvalue)
    (Class|IHUD|SetHP(Message) _widgetplayerpc (/ (Variables|Default|GetTempHP) (.CurrentValue (Utilities|Struct|BreakGameplayAttributeData (Variables|/Script/Boxing.MyAttributeSet|GetMaxHealth _attributeset)))))
    (else
      (Variables|Default|SetTempHP 0.0)
      (Class|IHUD|SetHP(Message) _widgetplayerpc (/ (Variables|Default|GetTempHP) (.CurrentValue (Utilities|Struct|BreakGameplayAttributeData (Variables|/Script/Boxing.MyAttributeSet|GetMaxHealth _attributeset)))))))
  (Class|MyCharacterBase|UpdateHP (Variables|Default|GetTempHP)))

(fn ConstructionScript
  (|CallParentFunction))

(fn JumpSectionforCombo
  (bind _ns_jumpsection (Variables|Combo|GetNS_JumpSection))
  (bind _mesh (Variables|Character|GetMesh))
  (bind _returnvalue (Components|SkeletalMesh|GetAnimInstance _mesh))
  (bind _jumpsections (Variables|/Game/Boxing/Characters/Animations/AnimNotifies/NS_JumpSection.NS_JumpSection_C|GetJumpSections _ns_jumpsection))
  (bind _returnvalue_2 (Animation|Montage|GetCurrentActiveMontage _returnvalue))
  (Utilities|IsValid _ns_jumpsection
    (:Is%20Valid
      (if (Variables|Combo|GetbEnableComboPeriod)
        (Class|AnimInstance|MontageSetNextSection _returnvalue (Animation|Montage|MontageGetCurrentSection _returnvalue _returnvalue_2) (Utilities|Array|Get(acopy) _jumpsections (Math|Random|RandomInteger (Utilities|Array|Length _jumpsections))) _returnvalue_2)
        (Variables|Combo|SetbEnableComboPeriod false)
        (return true)))))

(fn IsUsingMelee
  ;[1 1 1] 暂弃
  (bind _activeabilities (Class|MyCharacterBase|GetActiveAbilitieswithTags "(GameplayTags=((TagName=\"Event.Montage\")))"))
  (return (> (Utilities|Array|Length _activeabilities) 0)))

(fn Init
  (|CallParentFunction)
  (bind _asbp_player_controller (Utilities|Casting|CastToBP_PlayerController (Pawn|GetController)))
  (Utilities|IsValid (Variables|/Game/Boxing/Blueprints/Player/BP_PlayerController.BP_PlayerController_C|GetWidget_Player_PC _asbp_player_controller)
    (:Is%20Valid
      (Variables|Default|SetWidgetPlayerPC (Variables|/Game/Boxing/Blueprints/Player/BP_PlayerController.BP_PlayerController_C|GetWidget_Player_PC _asbp_player_controller)))))

(fn MeleeAttack
  (if (Variables|Combo|GetbEnableComboPeriod)
    (Development|PrintString "usingmelee is true")
    (CallFunction|JumpSectionforCombo)
    (return true)
    (else
      (Variables|Default|SetCurrentGameplayTag "(TagName=\"Event.Montage.Shared.MeleeHit\")")
      (Variables|Default|SetIsUsingMelee true)
      (Abilities|TryActivateAbilitybyClass (Variables|Default|GetAbilitySystemComponent) "/Game/Boxing/Abilities/player/GA_PlayerMelee.GA_PlayerMelee_C" true)
      (return true))))