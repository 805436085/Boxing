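; Base player character Blueprint for the boxing game, mapping player input to melee attack and jump actions.
; Fist and Foot presses share one path into PreMeleeAttack, with an authority switch whose branches are empty, while Jump calls DoJump.
; BeginPlay defers to the parent, and Init, InitBoxCollision and the construction script are empty.
; MeleeAttack and JumpSectionForCombo are stubs that only return true.
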(event Custom|Init)

(event EventBeginPlay
  (|CallParentFunction))

(event EventTick
  (params (DeltaSeconds :type Float%20%28single-precision%29)))

(event Input|ActionEvents|InputActionFist
  (params (Key :type Key%20Structure :default "None"))
  (:Pressed
    (Networking|SwitchHasAuthority
      (:Authority
        _)
      (:Remote
        _))
    (Class|MyCharacterBase|PreMeleeAttack)))

(event Input|ActionEvents|InputActionFoot
  (params (Key :type Key%20Structure :default "None"))
  (:Pressed
    (Networking|SwitchHasAuthority
      (:Authority
        _)
      (:Remote
        _))
    (Class|MyCharacterBase|PreMeleeAttack)))

(event Input|ActionEvents|InputActionJump
  (params (Key :type Key%20Structure :default "None"))
  (:Pressed
    (CallFunction|DoJump)))

(event EventInitBoxCollision)

(fn ConstructionScript)

(fn MeleeAttack
  (return true))

(fn JumpSectionforCombo
  (return true))