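; Flying sword weapon actor that rises on spawn, pauses briefly, then launches through ProjectileMovement.
; A timeline drives the lift and caches the Instigator as a BP_CharacterBase.
; Cone overlaps on other characters, filtered by a hit array and DoOnce, send the instigator's CurrentGameplayTag as a gameplay event with the target in its payload.
; HandBox_R end overlap with a player character resets the DoOnce.
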(event EventBeginPlay
  (bind _returnvalue (Transformation|GetActorLocation))
  (|CallParentFunction)
  (bind _新建轨道_0 (Timeline|时间轴_0 PlayFromStart)
    (:Update
      (Transformation|SetActorLocation (Math|Vector|MakeVector (.x _returnvalue) (.y _returnvalue) (Math|Float|Lerp (.z _returnvalue) (+ (.z _returnvalue) 1.0) _新建轨道_0)) true false)
      (bind _asbp_character_base (Utilities|Casting|CastToBP_CharacterBase (Variables|Default|GetInstigator)))
      (Variables|Default|SetSelfInstigator _asbp_character_base))
    (:Finished
      (Utilities|FlowControl|Delay 0.2)
      (Components|Activation|SetActive (Variables|Default|GetProjectileMovement) true false))))

(event Collision|EventActorBeginOverlap
  (params (OtherActor :type Actor%20Object%20Reference))
  (|CallParentFunction OtherActor) ; 此节点被禁用，将不会被调用。\n从引脚连出引线来编译功能。
)

(event EventTick
  (params (DeltaSeconds :type Float%20%28single-precision%29))
  (|CallParentFunction DeltaSeconds) ; 此节点被禁用，将不会被调用。\n从引脚连出引线来编译功能。
)

(event OnComponentBeginOverlap(Cone)
  (params (OverlappedComponent :type Primitive%20Component%20Object%20Reference) (OtherActor :type Actor%20Object%20Reference) (OtherComp :type Primitive%20Component%20Object%20Reference) (OtherBodyIndex :type Integer) (bFromSweep :type Boolean) (SweepResult :type Hit%20Result%20Structure%20%28by%20ref%29))
  (bind _selfinstigator (Variables|Default|GetSelfInstigator))
  (bind _collisiontargetarray (Variables|Default|GetCollisionTargetArray))
  (bind _currentgameplaytag (Variables|/Script/Boxing.MyCharacterBase|GetCurrentGameplayTag _selfinstigator))
  (if (!= OtherActor (Variables|Default|GetInstigator))
    (bind _asbp_character_base (Utilities|Casting|CastToBP_CharacterBase OtherActor))
    (Variables|Default|SetTargetActor _asbp_character_base)
    ;[1 1 1] 防穿模重入同一对象，本次攻击结束后清除
    (if (not (Utilities|Array|ContainsItem _collisiontargetarray (Variables|Default|GetTargetActor)))
      (Utilities|Array|Add _collisiontargetarray (Variables|Default|GetTargetActor))
      (Utilities|FlowControl|DoOnce false
        (:Completed
          (Utilities|IsValid _selfinstigator
            (:Is%20Valid
              (Ability|SendGameplayEventtoActor _selfinstigator _currentgameplaytag (Utilities|Struct|MakeGameplayEventData _currentgameplaytag _selfinstigator (Variables|Default|GetTargetActor)))
              (Development|PrintString "FlySword"))))))))

(event OnComponentEndOverlap(HandBox_R)
  (params (OverlappedComponent :type Primitive%20Component%20Object%20Reference) (OtherActor :type Actor%20Object%20Reference) (OtherComp :type Primitive%20Component%20Object%20Reference) (OtherBodyIndex :type Integer))
  (bind _selfinstigator (Variables|Default|GetSelfInstigator))
  (bind _currentgameplaytag (Variables|/Script/Boxing.MyCharacterBase|GetCurrentGameplayTag _selfinstigator))
  (Utilities|Casting|CastToBP_PlayerCharacterBase OtherActor)
  (Utilities|FlowControl|DoOnce false) ; enters at Reset
)

(fn ConstructionScript
  (|CallParentFunction))